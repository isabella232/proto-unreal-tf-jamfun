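; BP_Particles is an actor that drives a Niagara particle effect to follow the mouse cursor.
; Each tick it projects the cursor into the world at a fixed distance along the view ray and eases a stored location toward that point by Speed scaled with delta time.
; The smoothed location is passed to the Niagara component as the User.MousePosition vector parameter.
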(event EventBeginPlay)

(event Collision|EventActorBeginOverlap
  (params (OtherActor :type Actor%20Object%20Reference)))

(event EventTick
  (params (DeltaSeconds :type Float%20%28single-precision%29))
  (bind _returnvalue (Game|GetPlayerController 0))
  (bind (_worldlocation _worlddirection) (Game|Player|ConvertMouseLocationToWorldSpace _returnvalue))
  (bind _output_get (Variables|Default|SetCurrentLocation%20 (Math|Vector|Lerp(Vector) (Variables|Default|GetCurrentLocation%20) (+ _worldlocation (* _worlddirection 4.5e+02)) (* (Variables|Default|GetSpeed) (Utilities|Time|GetWorldDeltaSeconds)))))
  (Class|NiagaraComponent|SetNiagaraVariableVec3 (Variables|Default|GetNiagara) "User.MousePosition" _output_get))

(fn ConstructionScript)