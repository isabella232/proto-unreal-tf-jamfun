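; UI cine camera that shifts around its starting location to follow a centered screen-space target, likely the cursor, for a parallax-style view.
; BeginPlay stores the initial location; each Tick, GetScreenInfo supplies the target, with a MoveOnlyOnClick option.
; GetLocationFromOffset2D turns it into a new location using Multiplier and Speed, feeding the current offset back each frame before the actor moves without sweeping.
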(event EventBeginPlay
  (Variables|Default|SetInitial%20Location (Transformation|GetActorLocation)))

(event EventTick
  (params (DeltaSeconds :type Float%20%28single-precision%29))
  (bind (_x _y _normalizedx _normalizedy _centeredx _centeredy) (CallFunction|GetScreenInfo (Variables|CameraMovement|GetMoveOnlyOnClick)))
  (bind (_newlocation _newx _newy) (CallFunction|GetLocationfromOffset2D (Variables|Default|GetInitial%20Location) (Variables|Default|GetCurrentX) (Variables|Default|GetCurrentY) _centeredx _centeredy (Variables|CameraMovement|GetMultiplier) (Variables|CameraMovement|GetSpeed)))
  (Variables|Default|SetCurrentX _newx)
  (Variables|Default|SetCurrentY _newy)
  (Transformation|SetActorLocation _newlocation false false))

(fn ConstructionScript)