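; Blueprint helper functions for UI view movement driven by the mouse position.
; GetScreenInfo returns raw, normalized and centered (-1 to 1) cursor coordinates, zeroing the centered values when invalid or, optionally, when Touch1 is not pressed.
; GetLocationFromOffset2D lerps an X/Y offset toward a target using delta time and applies it to an initial location's X and Z.
; SetLookAt rotates an actor toward another actor plus an offset.
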(fn GetScreenInfo
  (params (OnlyOnClick :type Boolean))
  (bind _returnvalue (Game|GetPlayerController 0))
  (bind _returnvalue_2 (Viewport|GetViewportSize))
  (bind (_locationx _locationy _returnvalue_3) (Game|Player|GetMousePosition _returnvalue))
  (bind _biscurrentlypressed (Class|PlayerController|GetInputTouchState _returnvalue "Touch1"))
  (bind (_x _y) (Math|Vector2D|BreakVector2D _returnvalue_2))
  (bind _returnvalue_4 (/ _locationx _x))
  (bind _returnvalue_5 (/ _locationy _y))
  (bind _returnvalue_6 (select OnlyOnClick _biscurrentlypressed true))
  (bind _returnvalue_7 (and _returnvalue_3 _returnvalue_6))
  (return _locationx _locationy _returnvalue_4 _returnvalue_5 (Math|Float|SelectFloat (- (* _returnvalue_4 2.0) 1.0) 0.0 _returnvalue_7) (Math|Float|SelectFloat (- (* _returnvalue_5 2.0) 1.0) 0.0 _returnvalue_7) _returnvalue_7))

(fn SetLookat
  (params (Target :type Actor%20Object%20Reference) (LookAtTarget :type Actor%20Object%20Reference) (Offset :type Vector))
  (Utilities|IsValid LookAtTarget
    (:Is%20Valid
      (Transformation|SetActorRotation Target (Math|Rotator|FindLookatRotation (Transformation|GetActorLocation Target) (+ (Transformation|GetActorLocation LookAtTarget) Offset))))))

(fn GetLocationfromOffset2D
  (params (InitialLocation :type Vector) (CurrentX :type Float%20%28single-precision%29) (CurrentY :type Float%20%28single-precision%29) (TargetX :type Float%20%28single-precision%29) (TargetY :type Float%20%28single-precision%29) (Multiplier :type Vector%202D%20Structure) (Speed :type Vector%202D%20Structure))
  (bind _returnvalue (Utilities|Time|GetWorldDeltaSeconds))
  (bind (_x _y) (Math|Vector2D|BreakVector2D Multiplier))
  (bind (_x_2 _y_2) (Math|Vector2D|BreakVector2D Speed))
  (bind (_x_3 _y_3 _z) (Math|Vector|BreakVector InitialLocation))
  (bind _returnvalue_2 (* _x_2 _returnvalue))
  (bind _returnvalue_3 (* _y_2 _returnvalue))
  (bind _returnvalue_4 (Math|Float|Lerp CurrentY TargetY _returnvalue_3))
  (bind _returnvalue_5 (Math|Float|Lerp CurrentX TargetX _returnvalue_2))
  (return (Math|Vector|MakeVector (+ _x_3 (* _x _returnvalue_5)) _y_3 (+ _z (* _y _returnvalue_4))) _returnvalue_5 _returnvalue_4))