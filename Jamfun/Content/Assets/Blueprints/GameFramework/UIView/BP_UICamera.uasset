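; BP_UICamera is a UI view camera that shifts around its starting location in response to centered screen coordinates while aiming at a target actor.
; BeginPlay stores the initial location.
; Each Tick, GetScreenInfo, configured by OnlyMoveOnClick, supplies centered X/Y targets to GetLocationFromOffset2D, which uses Multiplier and Speed to compute the new position.
; The current offsets carry between frames, and SetLookAt re-aims at LookAtTargetActor with TargetOffset after each move.
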(event EventBeginPlay
  (Variables|Default|SetInitialLocation (Transformation|GetActorLocation)))

(event EventTick
  (params (DeltaSeconds :type Float%20%28single-precision%29))
  (bind (_x _y _normalizedx _normalizedy _centeredx _centeredy) (CallFunction|GetScreenInfo (Variables|CameraMouseMovement|GetOnlyMoveOnClick)))
  (bind (_newlocation _newx _newy) (CallFunction|GetLocationfromOffset2D (Variables|Default|GetInitialLocation) (Variables|Default|GetCurrentX) (Variables|Default|GetCurrentY) _centeredx _centeredy (Variables|CameraMouseMovement|GetMultiplier) (Variables|CameraMouseMovement|GetSpeed)))
  (Variables|Default|SetCurrentX _newx)
  (Variables|Default|SetCurrentY _newy)
  (Transformation|SetActorLocation _newlocation false false)
  (CallFunction|SetLookat self (Variables|CameraMouseMovement|GetLookAtTargetActor) (Variables|CameraMouseMovement|GetTargetOffset)))

(fn ConstructionScript)