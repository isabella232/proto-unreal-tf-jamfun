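; BP_LIghtParticles is an environment Blueprint that moves a mesh and a light to trail the player's mouse cursor through the world.
; Each Tick it deprojects the first player controller's mouse position and projects a target a fixed distance along that ray.
; A stored location lerps toward the target by Speed scaled with delta time, giving eased motion, then sets both components' world locations without sweeping.
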(event EventBeginPlay)

(event EventTick
  (params (DeltaSeconds :type Float%20%28single-precision%29))
  (bind _returnvalue (Game|GetPlayerController 0))
  (bind (_worldlocation _worlddirection) (Game|Player|ConvertMouseLocationToWorldSpace _returnvalue))
  (bind _output_get (Variables|Default|SetCurrentLocation (Math|Vector|Lerp(Vector) (Variables|Default|GetCurrentLocation) (+ _worldlocation (* _worlddirection 4.5e+02)) (* (Variables|Default|GetSpeed) (Utilities|Time|GetWorldDeltaSeconds)))))
  (Transformation|SetWorldLocation (Variables|Default|Getmesh) _output_get false false))

(fn ConstructionScript)